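; BP_character is a character Blueprint that handles basic player movement and jumping from input.
; MoveForward and MoveRight axes add movement input along control-rotation yaw directions, scaled by a Speed variable.
; Either Shift key raises Speed to full while held and halves it on release, changing input scale rather than the movement component's max speed.
; The Jump action calls the built-in Jump, and the construction script is empty.
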(event Input|ActionEvents|InputActionJump
  (params (Key :type Key%20Structure))
  ;[1 1 1] ジャンプ
  (:Pressed
    (Character|Jump)))

(event Input|AxisEvents|InputAxisMoveForward
  (params (AxisValue :type Float%20%28single-precision%29))
  ;[1 1 1] キャラクターの移動
  (Pawn|Input|AddMovementInput (Math|Vector|GetForwardVector (Math|Rotator|MakeRotator 0.0 0.0 (.Yaw (Math|Rotator|BreakRotator (Pawn|GetControlRotation :!class /Script/Engine.Pawn))))) (* AxisValue (Variables|Default|GetSpeed)) false))

(event Input|AxisEvents|InputAxisMoveRight
  (params (AxisValue :type Float%20%28single-precision%29))
  ;[1 1 1] キャラクターの移動
  (Pawn|Input|AddMovementInput (Math|Vector|GetRightVector (Math|Rotator|MakeRotator 0.0 0.0 (.Yaw (Math|Rotator|BreakRotator (Pawn|GetControlRotation :!class /Script/Engine.Pawn))))) (* AxisValue (Variables|Default|GetSpeed)) false))

(event Input|KeyboardEvents|LeftShift
  (params (Key :type Key%20Structure))
  ;[1 1 1] shiftでの移動速度変更
  (:Pressed
    (Variables|Default|SetSpeed 1.0))
  (:Released
    (Variables|Default|SetSpeed 0.5)))

(event Input|KeyboardEvents|RightShift
  (params (Key :type Key%20Structure))
  ;[1 1 1] shiftでの移動速度変更
  (:Pressed
    (Variables|Default|SetSpeed 1.0))
  (:Released
    (Variables|Default|SetSpeed 0.5)))

(fn ConstructionScript)